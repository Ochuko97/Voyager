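; Test cube actor that gives itself a random colour when it spawns and destroys itself after a fixed lifespan.
; BeginPlay sets the lifespan, then switches on a random integer to apply a red, blue, yellow or green material to the Cube component.
; Each branch stores a matching number in ColourID, which nothing in this Blueprint reads.
; The construction script is empty.
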(event EventBeginPlay
  (Actor|SetLifeSpan 1e+02)
  (switch int (Math|Random|RandomIntegerinRange 0 3)
    (:0
      (Rendering|Material|SetMaterial (Variables|Default|GetCube) 0 "/Game/Assets/Materia/Spirits/Red.Red")
      ;[1 1 1] Red is 1
      (Variables|Default|SetColourID 1))
    (:1
      (Rendering|Material|SetMaterial (Variables|Default|GetCube) 0 "/Game/Assets/Materia/Spirits/Blue.Blue")
      ;[1 1 1] Blue is 2
      (Variables|Default|SetColourID 2))
    (:2
      (Rendering|Material|SetMaterial (Variables|Default|GetCube) 0 "/Game/Assets/Materia/Spirits/Yellow.Yellow")
      ;[1 1 1] Yellow is 3
      (Variables|Default|SetColourID 3))
    (:3
      (Rendering|Material|SetMaterial (Variables|Default|GetCube) 0 "/Game/Assets/Materia/Spirits/Green.Green")
      ;[1 1 1] Green is 4
      (Variables|Default|SetColourID 4))))

(fn ConstructionScript)