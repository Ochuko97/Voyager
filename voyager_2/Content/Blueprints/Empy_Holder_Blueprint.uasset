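; Empy_Holder_Blueprint is an actor that the player shifts in fixed steps with the Up, Left and Right arrow keys.
; BeginPlay enables input from player controller 0, and each key calls its own movement event: forward on +Y, left on +X, right on -X.
; Each event uses MoveComponentTo with zero duration, instantly setting DefaultSceneRoot1's relative location to the actor's location plus the offset.
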(event Custom|Move%20Forward
  (Components|MoveComponentTo (Variables|Default|GetDefaultSceneRoot1) (+ (Transformation|GetActorLocation) "0,200.000000, 0") "0, 0, 0" true true 0.0 false))

(event Custom|Move%20Right
  (Components|MoveComponentTo (Variables|Default|GetDefaultSceneRoot1) (- (Transformation|GetActorLocation) "200.000000, 0, 0") "0, 0, 0" true true 0.0 false))

(event Custom|Move%20Left
  (Components|MoveComponentTo (Variables|Default|GetDefaultSceneRoot1) (+ (Transformation|GetActorLocation) "200.000000,0.000000, 0") "0, 0, 0" true true 0.0 false))

(event EventBeginPlay
  (Input|EnableInput (Game|GetPlayerController 0)))

(event Input|KeyboardEvents|Up
  (params (Key :type Key%20Structure))
  (:Pressed
    (CallFunction|MoveForward)))

(event Input|KeyboardEvents|Left
  (params (Key :type Key%20Structure))
  (:Pressed
    (CallFunction|MoveLeft)))

(event Input|KeyboardEvents|Right
  (params (Key :type Key%20Structure))
  (:Pressed
    (CallFunction|MoveRight)))

(fn ConstructionScript)